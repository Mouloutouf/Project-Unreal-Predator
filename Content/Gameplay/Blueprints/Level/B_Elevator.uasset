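; B_Elevator is a level elevator that activates on BeginPlay and moves its platform vertically.
; While active, it calls MoveElevator every tick, which plays or reverses the Move timeline depending on IsForward.
; The timeline's curve, scaled by Height, sets the platform's relative Z, and SwitchDirection runs when the timeline finishes.
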(event Custom|MoveElevator
  (if (Class|Elevator|IsForward)
    (bind _movecurve (Timeline|Move Play)
      (:Update
        (Transformation|SetRelativeLocation (Variables|Default|GetPlatform) (Math|Vector|MakeVector 0.0 0.0 (* _movecurve (Variables|Default|GetHeight))) false false))
      (:Finished
        (Class|Elevator|SwitchDirection)))
    (else
      (Timeline|Move Reverse))))

(event EventBeginPlay
  (Class|Elevator|SetActive true))

(event EventTick
  (params (DeltaSeconds :type Float%20%28single-precision%29))
  (if (Variables|Default|GetIsActive)
    (CallFunction|MoveElevator)))

(fn ConstructionScript)