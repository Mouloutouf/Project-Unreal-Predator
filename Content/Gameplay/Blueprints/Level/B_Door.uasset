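; B_Door is a sliding level door that opens for the player character when unlocked and can display its lock state as text.
; Trigger overlaps by B_PlayerCharacter play or reverse the DoorSlide timeline, which scales the door's starting relative Z to move it vertically.
; OnLockUpdated sets the label to LOCKED or UNLOCKED, or blanks it when ShowText is off.
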(event OnComponentBeginOverlap(DoorTrigger)
  (params (OverlappedComponent :type Primitive%20Component%20Object%20Reference) (OtherActor :type Actor%20Object%20Reference) (OtherComp :type Primitive%20Component%20Object%20Reference) (OtherBodyIndex :type Integer) (bFromSweep :type Boolean) (SweepResult :type Hit%20Result%20Structure%20%28by%20ref%29))
  (Utilities|Casting|CastToB_PlayerCharacter OtherActor)
  (if (Variables|Default|GetUnlocked)
    (bind _slide (Timeline|Door%20Slide Play)
      (:Update
        (Transformation|SetRelativeLocation (Variables|Default|GetSliding%20Door) (Math|Vector|MakeVector 0.0 0.0 (* _slide (Variables|Default|GetDoor%20Height))) false false)))))

(event OnComponentEndOverlap(DoorTrigger)
  (params (OverlappedComponent :type Primitive%20Component%20Object%20Reference) (OtherActor :type Actor%20Object%20Reference) (OtherComp :type Primitive%20Component%20Object%20Reference) (OtherBodyIndex :type Integer))
  (Utilities|Casting|CastToB_PlayerCharacter OtherActor)
  (if (Variables|Default|GetUnlocked)
    (bind _slide (Timeline|Door%20Slide Reverse)
      (:Update
        (Transformation|SetRelativeLocation (Variables|Default|GetSliding%20Door) (Math|Vector|MakeVector 0.0 0.0 (* _slide (Variables|Default|GetDoor%20Height))) false false)))))

(event EventBeginPlay
  (Variables|Default|SetDoor%20Height (.z (Variables|/Script/Engine.SceneComponent|GetRelativeLocation (Variables|Default|GetSliding%20Door))))
  (Class|Door|OnLockUpdated (Variables|Default|GetUnlocked)))

(event EventOnLockUpdated
  (params (bValue :type Boolean))
  (if (Variables|Default|GetShowText)
    (if bValue
      (Variables|Default|SetLockedText "UNLOCKED")
      (else
        (Variables|Default|SetLockedText "LOCKED")))
    (Rendering|Components|TextRender|SetText (Variables|Default|GetLocked%20Text) (Variables|Default|GetLockedText))
    (else
      (Rendering|Components|TextRender|SetText (Variables|Default|GetLocked%20Text) (Utilities|Text|MakeLiteralText "")))))

(fn ConstructionScript)